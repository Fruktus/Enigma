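; Glass letter actor that switches its mesh between a lit and a dark look.
; It applies the dark material to the first slot of its static mesh at BeginPlay.
; Each EventLight call flips the IsLight flag and swaps in the light or dark material to match, but only while ShouldShine is true.
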(event Custom|EventLight
  (if (Variables|Default|GetshouldShine)
    (bind _output_get (Variables|Default|SetisLight (not (Variables|Default|GetisLight))))
    (if _output_get
      (Rendering|Material|SetMaterial (Variables|Debug|GetStaticMeshComponent) 0 (Variables|Default|GetlightMaterial))
      (else
        (Rendering|Material|SetMaterial (Variables|Debug|GetStaticMeshComponent) 0 (Variables|Default|GetdarkMaterial))))))

(event EventBeginPlay
  (Rendering|Material|SetMaterial (Variables|Debug|GetStaticMeshComponent) 0 (Variables|Default|GetdarkMaterial)))

(event Collision|EventActorBeginOverlap
  (params (OtherActor :type Actor%20Object%20Reference)))

(event EventTick
  (params (DeltaSeconds :type Float%20%28single-precision%29)))

(fn ConstructionScript)