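; Draggable rotor actor for a socket-based machine, acting according to whether the SocketManager's top cover is open.
; With the cover open, a held rotor follows the deprojected mouse and on release plugs into the selected socket or returns to its own.
; With it closed, vertical dragging spins it with a randomly pitched click per step.
; Release stores the nearest integer offset and a timeline eases the rotation onto that step.
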(event EventBeginPlay
  (Variables|Default|SetstartRotation (Transformation|GetActorRotation)))

(event MouseInput|EventActorOnClicked
  (params (ButtonPressed :type Key%20Structure))
  (Variables|Default|SetisHeld true)
  (if (not (CallFunction|IsCoverOpen))
    (bind _returnvalue (Class|WidgetLayoutLibrary|GetMousePositiononViewport))
    (Variables|Default|SetmouseLastPos _returnvalue)))

(event EventTick
  (params (DeltaSeconds :type Float%20%28single-precision%29))
  (if (Variables|Default|GetisHeld)
    (if (CallFunction|IsCoverOpen) ; if open - swap, closed - rotate
      (CallFunction|SetPositiontoMouse)
      (else
        (CallFunction|SetRotationMouse)))))

(event EventAnimateNewOffset
  (params (rotation :type Float%20%28single-precision%29))
  (bind _startrotation (Variables|Default|GetstartRotation))
  (bind (_roll _pitch _yaw) (Math|Rotator|BreakRotator _startrotation))
  (Audio|PlaySound2D "/Game/Sounds/rotor-set.rotor-set" 1.0 (Math|Random|RandomFloatinRange 0.85 1.15) 0.0 0 0)
  (bind _newtrack_0 (Timeline|Timeline_1 PlayFromStart)
    (:Update
      (Transformation|SetActorRotation (Math|Rotator|Lerp(Rotator) (Transformation|GetActorRotation) (Math|Rotator|MakeRotator (- _roll rotation) _pitch _yaw) _newtrack_0 true)))))

(event Input|MouseEvents|LeftMouseButton
  (params (Key :type Key%20Structure))
  (bind _returnvalue (Transformation|GetActorRotation))
  (bind _roll (Math|Rotator|BreakRotator _returnvalue))
  (bind _absyrotation (CallFunction|GetAbsoluteRotation _roll))
  (bind _offset (CallFunction|GetIntOffset _absyrotation))
  (:Released
    (if (Variables|Default|GetisHeld)
      (Variables|Default|SetisHeld false)
      (if (CallFunction|IsCoverOpen)
        (if (Variables|/Game/Blueprints/rotorSocketManager.rotorSocketManager_C|GetisSocketSelected (Variables|Default|GetsocketManager))
          (Default|PlugIntoSocket (Variables|Default|GetsocketManager) self)
          (else
            (CallFunction|ReturntoBaseLocation)))
        (else
          (Class|Rotor|SetOffset _offset)
          (Class|Rotor|AnimateNewOffset (* _offset (Variables|Default|GetstepDegree))))))))

(fn ConstructionScript
  (bind _stepdegree (CallFunction|GetStepDegree))
  (Variables|Default|SetstepDegree _stepdegree))

(fn GetStepDegree
  (return (/ 3.6e+02 (Math|Conversions|ToFloat(Integer) (Variables|Default|Getmax_rotates)))))

(fn IsCoverOpen
  (return (Variables|/Game/Blueprints/topCover_Blueprint.topCover_Blueprint_C|GetisOpen (Variables|/Game/Blueprints/rotorSocketManager.rotorSocketManager_C|GettopCover (Variables|Default|GetsocketManager)))))

(fn GetRotationMovedbyDiff
  (params (difference :type Float%20%28single-precision%29))
  (return (Math|Rotator|MakeRotator (* (/ difference (* (.y (Viewport|GetViewportSize)) 0.04)) -7.0) 0.0 0.0) (Transformation|GetActorRotation)))

(fn TrytoPlayClickSound
  (params (NewRotation :type Rotator) (OldRotation :type Rotator))
  (if (== (CallFunction|GetIntOffset (.Roll (Math|Rotator|BreakRotator NewRotation))) (CallFunction|GetIntOffset (.Roll (Math|Rotator|BreakRotator OldRotation))))
    _
    (else
      (Audio|PlaySound2D "/Game/Sounds/rotor-set.rotor-set" 1.0 (Math|Random|RandomFloatinRange 0.85 1.15) 0.0 0 0)))
  (return))

(fn GetIntOffset
  (params (YRotation :type Float%20%28single-precision%29))
  (return (Math|Float|Round (/ YRotation (Variables|Default|GetstepDegree)))))

(fn AnimateOffsetChangeRotation
  (params (offsetDegree :type Float%20%28single-precision%29) (alpha :type Float%20%28single-precision%29))
  (bind _startrotation (Variables|Default|GetstartRotation))
  (bind (_roll _pitch _yaw) (Math|Rotator|BreakRotator _startrotation))
  (return (Math|Rotator|Lerp(Rotator) (Transformation|GetActorRotation) (Math|Rotator|MakeRotator (+ offsetDegree _roll) _pitch _yaw) alpha true)))

(fn GetAbsoluteRotation
  (params (YRotation :type Float%20%28single-precision%29))
  (return (- (.Roll (Math|Rotator|BreakRotator (Variables|Default|GetstartRotation))) YRotation)))

(fn SetPositiontoMouse
  (bind _returnvalue (Class|WidgetLayoutLibrary|GetMousePositiononViewport))
  (Transformation|SetWorldLocation (Variables|Default|GetDefaultSceneRoot) (+ (+ (.WorldPosition (Class|GameplayStatics|DeprojectScreentoWorld (Game|GetPlayerController 0) (Utilities|ScaleMousePos _returnvalue))) (* (.WorldDirection (Class|GameplayStatics|DeprojectScreentoWorld (Game|GetPlayerController 0) (Utilities|ScaleMousePos _returnvalue))) 5e+02)) (Math|Vector|MakeVector 0.0 (* 5e+01 (Utilities|GetDPIScale)) 0.0)) false false))

(fn SetRotationMouse
  (bind _returnvalue (Class|WidgetLayoutLibrary|GetMousePositiononViewport))
  (if (not (== (.Y (Math|Vector2D|BreakVector2D _returnvalue)) (.Y (Math|Vector2D|BreakVector2D (Variables|Default|GetmouseLastPos)))))
    (bind (_deltarotatio _oldrotation) (CallFunction|GetRotationMovedbyDiff (- (.Y (Math|Vector2D|BreakVector2D _returnvalue)) (.Y (Math|Vector2D|BreakVector2D (Variables|Default|GetmouseLastPos))))))
    (Transformation|AddActorLocalRotation _deltarotatio false false)
    (CallFunction|TrytoPlayClickSound (Transformation|GetActorRotation) _oldrotation)
    (Variables|Default|SetmouseLastPos _returnvalue)))

(fn ReturntoBaseLocation
  (bind _socket (Default|GetRotorSocket (Variables|Default|GetsocketManager) self))
  (Transformation|SetWorldLocation (Variables|Default|GetDefaultSceneRoot) (Transformation|GetWorldLocation (Variables|/Game/Blueprints/rotorSocket.rotorSocket_C|GetDefaultSceneRoot _socket)) false false))