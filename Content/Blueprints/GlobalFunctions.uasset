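; Blueprint function library that converts between the ELetter enum and single-character strings.
; Both functions index into the character array of a shared TranslationString, so each enum value maps to the character at the same position.
; StringToELetter uppercases its input before searching, making the lookup case-insensitive for lowercase letters.
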(fn ELettertoString
  (params (Letter :type ELetter%20Enum :default "A"))
  (return (Utilities|Array|Get(acopy) (Utilities|String|GetCharacterArrayfromString (LocalVariables|GettranslationString)) (Math|Conversions|ToInteger(Byte) Letter))))

(fn StringtoELetter
  (params (StringLetter :type String))
  (return (Utilities|Enum|ByteToEnumELetter (Math|Conversions|ToByte(Integer) (Utilities|Array|FindItem (Utilities|String|GetCharacterArrayfromString (LocalVariables|GettranslationString)) (Class|KismetStringLibrary|ToUpper StringLetter))))))