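; Plugboard cable with two draggable plugs that pairs socket letters for a letter-substitution encoding.
; Clicking a plug unplugs it through Sb, then Tick moves it with the deprojected mouse at a fixed depth until release snaps it to the selected socket.
; BeginPlay seats default plugs, though both store into Plug1Letter, and briefly hides the cable.
; GetEncoding swaps the connected letters, passing others through unchanged.
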(event OnClicked(plug2)
  (params (TouchedComponent :type Primitive%20Component%20Object%20Reference) (ButtonPressed :type Key%20Structure))
  (Variables|Default|SetplugHeld (Variables|Default|Getplug2))
  (Default|Unplug (Variables|Default|Getsb) (Variables|Default|Getplug2Letter))
  (Variables|Default|Setplug2Letter "None")
  (Variables|Default|SetisPlugHeld true)
  (Variables|/Game/Blueprints/Switchboard-Blueprint.Switchboard-Blueprint_C|Setenabled (Variables|Default|Getsb) true)
  (Audio|PlaySound2D "/Game/Sounds/plug.plug" 1.0 (Math|Random|RandomFloatinRange 0.85 1.15) 0.0 0 0))

(event OnClicked(plug1)
  (params (TouchedComponent :type Primitive%20Component%20Object%20Reference) (ButtonPressed :type Key%20Structure))
  (Variables|Default|SetplugHeld (Variables|Default|Getplug1))
  (Default|Unplug (Variables|Default|Getsb) (Variables|Default|Getplug1Letter))
  (Variables|Default|Setplug1Letter "None")
  (Variables|Default|SetisPlugHeld true)
  (Variables|/Game/Blueprints/Switchboard-Blueprint.Switchboard-Blueprint_C|Setenabled (Variables|Default|Getsb) true)
  (Audio|PlaySound2D "/Game/Sounds/plug.plug" 1.0 (Math|Random|RandomFloatinRange 0.85 1.15) 0.0 0 0))

(event EventBeginPlay
  (Rendering|SetVisibility (Variables|Default|GetCable) false false)
  (if (Utilities|Name|Equal(Name) (Variables|Default|Getplug1DefSocket) "None")
    _
    (else
      (bind _socketlocation (Default|GetSocketLocationbyName (Variables|Default|Getsb) (Variables|Default|Getplug1DefSocket)))
      (Transformation|SetWorldLocation (Variables|Default|Getplug1) (+ _socketlocation "-20.000000,0.000000,-10.000000") false false)
      (bind _letter (Default|Plug (Variables|Default|Getsb) self (Variables|Default|Getplug1DefSocket)))
      (Variables|Default|Setplug1Letter _letter)))
  (if (Utilities|Name|Equal(Name) (Variables|Default|Getplug2DefSocket) "None")
    _
    (else
      (bind _socketlocation_2 (Default|GetSocketLocationbyName (Variables|Default|Getsb) (Variables|Default|Getplug2DefSocket)))
      (Transformation|SetWorldLocation (Variables|Default|Getplug2) (+ _socketlocation_2 "-20.000000,0.000000,-10.000000") false false)
      (bind _letter_2 (Default|Plug (Variables|Default|Getsb) self (Variables|Default|Getplug2DefSocket)))
      (Variables|Default|Setplug1Letter _letter_2)))
  (Utilities|FlowControl|Delay 1.0)
  (Rendering|SetVisibility (Variables|Default|GetCable) true false))

(event EventTick
  (params (DeltaSeconds :type Float%20%28single-precision%29))
  (if (and (Variables|Default|GetisPlugHeld) (Variables|Default|Getactive))
    (bind _returnvalue (Class|WidgetLayoutLibrary|GetMousePositiononViewport))
    (Transformation|SetWorldLocation (Variables|Default|GetplugHeld) (Math|Vector|MakeVector (Variables|Default|GetheldDepth) (+ (.y (+ (.WorldPosition (Class|GameplayStatics|DeprojectScreentoWorld (Game|GetPlayerController 0) (* _returnvalue (Utilities|GetDPIScale)))) (* (.WorldDirection (Class|GameplayStatics|DeprojectScreentoWorld (Game|GetPlayerController 0) (* _returnvalue (Utilities|GetDPIScale)))) (Math|Float|Absolute(Float) (- -6.5e+02 (Variables|Default|GetheldDepth)))))) (* 1e+01 (Utilities|GetDPIScale))) (.z (+ (.WorldPosition (Class|GameplayStatics|DeprojectScreentoWorld (Game|GetPlayerController 0) (* _returnvalue (Utilities|GetDPIScale)))) (* (.WorldDirection (Class|GameplayStatics|DeprojectScreentoWorld (Game|GetPlayerController 0) (* _returnvalue (Utilities|GetDPIScale)))) (Math|Float|Absolute(Float) (- -6.5e+02 (Variables|Default|GetheldDepth))))))) false false)))

(event Input|MouseEvents|LeftMouseButton
  (params (Key :type Key%20Structure))
  (bind _sb (Variables|Default|Getsb))
  (:Released
    (Variables|/Game/Blueprints/Switchboard-Blueprint.Switchboard-Blueprint_C|Setenabled (Variables|Default|Getsb) false)
    (if (Math|Boolean|ANDBoolean (Variables|Default|GetisPlugHeld) (Variables|Default|Getactive) (Variables|/Game/Blueprints/Switchboard-Blueprint.Switchboard-Blueprint_C|GetsocketSelected _sb))
      (Transformation|SetWorldLocation (Variables|Default|GetplugHeld) (+ (Variables|/Game/Blueprints/Switchboard-Blueprint.Switchboard-Blueprint_C|GetclosestSocketLocation3D _sb) "-20.000000,0.000000,-10.000000") false false)
      (bind _letter (Default|Plug (Variables|Default|Getsb) self "None"))
      (Audio|PlaySound2D "/Game/Sounds/plug.plug" 1.0 (Math|Random|RandomFloatinRange 0.85 1.15) 0.0 0 0)
      (if (== (Variables|Default|GetplugHeld) (Variables|Default|Getplug1))
        (Variables|Default|Setplug1Letter _letter)
        (else
          (Variables|Default|Setplug2Letter _letter))))
    (Variables|Default|SetisPlugHeld false)))

(fn ConstructionScript)

(fn GetEncoding
  (params (letter :type String))
  (if (Utilities|Enum|Equal(Enum) letter (Variables|Default|Getplug1Letter))
    (if (Utilities|Enum|Equal(Enum) (Variables|Default|Getplug2Letter) "None")
      _
      (else
        (return (Variables|Default|Getplug2Letter))))
    (elif (Utilities|Enum|Equal(Enum) (Variables|Default|Getplug2Letter) letter)
      (if (Utilities|Enum|Equal(Enum) "None" (Variables|Default|Getplug1Letter))
        _
        (else
          (return (Variables|Default|Getplug1Letter))))))
  (return letter))