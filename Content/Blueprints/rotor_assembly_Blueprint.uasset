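; Rotor actor that turns in discrete steps and carries over to a linked rotor, like an odometer.
; Each RotateEvent increments a counter and plays a timeline that lerps pitch by one MaxRotates fraction of a full turn, offset from the rotation saved at BeginPlay.
; When the count reaches MaxRotates it resets and triggers NextRotor, if valid, to step once.
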(event Custom|Rotate%20Event
  (bind _startrotation (Variables|Default|GetstartRotation))
  (bind _max_rotates (Variables|Default|Getmax_rotates))
  (bind _returnvalue (Math|Conversions|ToFloat(Integer) _max_rotates))
  (bind (_roll _pitch _yaw) (Math|Rotator|BreakRotator _startrotation))
  (bind _returnvalue_2 (/ 3.6e+02 _returnvalue))
  (bind _result (Math|Integer|IncrementInt (Variables|Default|Getrotates_count))
    (:%20%20
      (CallFunction|RotateNext)
      (bind _newtrack_0 (Timeline|RotateTimeline PlayFromStart)
        (:Update
          (Transformation|SetActorRotation (Math|Rotator|MakeRotator _roll (+ (Math|Float|Lerp (* (Math|Conversions|ToFloat(Integer) (- _result 1)) _returnvalue_2) (* (Math|Conversions|ToFloat(Integer) _result) _returnvalue_2) _newtrack_0) _pitch) _yaw)))))))

(event Custom|Rotate%20Next
  (if (>= (Variables|Default|Getrotates_count) (Variables|Default|Getmax_rotates))
    (Variables|Default|Setrotates_count 0)
    (Utilities|IsValid (Variables|Default|Getnext_rotor)
      (:Is%20Valid
        (CallFunction|RotateEvent (Variables|Default|Getnext_rotor))))))

(event EventBeginPlay
  (Variables|Default|SetstartRotation (Transformation|GetActorRotation)))

(fn ConstructionScript)