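; Cable actor with two draggable plugs that pairs two letters for an encoding, in the manner of an Enigma plugboard.
; Clicking a plug unplugs it via Sb, and Tick moves it with the deprojected, DPI-scaled mouse position at a fixed depth while Active.
; Releasing the mouse centers it on any selected socket and stores the letter Sb returns.
; GetEncoding returns the opposite plug's letter, or the input if that end is unplugged.
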(event OnClicked(plug2)
  (params (TouchedComponent :type Primitive%20Component%20Object%20Reference) (ButtonPressed :type Key%20Structure))
  (Variables|Default|SetplugHeld (Variables|Default|Getplug2))
  (Default|Unplug (Variables|Default|Getsb) (Variables|Default|Getplug2Letter))
  (Variables|Default|Setplug2Letter "None")
  (Variables|Default|SetisPlugHeld true)
  (Variables|/Game/Blueprints/Switchboard_Blueprint.Switchboard_Blueprint_C|Setenabled (Variables|Default|Getsb) true))

(event OnClicked(plug1)
  (params (TouchedComponent :type Primitive%20Component%20Object%20Reference) (ButtonPressed :type Key%20Structure))
  (Variables|Default|SetplugHeld (Variables|Default|Getplug1))
  (Default|Unplug (Variables|Default|Getsb) (Variables|Default|Getplug1Letter))
  (Variables|Default|Setplug1Letter "None")
  (Variables|Default|SetisPlugHeld true)
  (Variables|/Game/Blueprints/Switchboard_Blueprint.Switchboard_Blueprint_C|Setenabled (Variables|Default|Getsb) true))

(event EventTick
  (params (DeltaSeconds :type Float%20%28single-precision%29))
  (if (and (Variables|Default|GetisPlugHeld) (Variables|Default|Getactive))
    (bind _returnvalue (Class|WidgetLayoutLibrary|GetMousePositiononViewport))
    (Transformation|SetWorldLocation (Variables|Default|GetplugHeld) (Math|Vector|MakeVector (Variables|Default|GetheldDepth) (.y (+ (.WorldPosition (Class|GameplayStatics|DeprojectScreentoWorld (Game|GetPlayerController 0) (* _returnvalue (Utilities|GetDPIScale)))) (* (.WorldDirection (Class|GameplayStatics|DeprojectScreentoWorld (Game|GetPlayerController 0) (* _returnvalue (Utilities|GetDPIScale)))) (Math|Float|Absolute(Float) (- -6.5e+02 (Variables|Default|GetheldDepth)))))) (.z (+ (.WorldPosition (Class|GameplayStatics|DeprojectScreentoWorld (Game|GetPlayerController 0) (* _returnvalue (Utilities|GetDPIScale)))) (* (.WorldDirection (Class|GameplayStatics|DeprojectScreentoWorld (Game|GetPlayerController 0) (* _returnvalue (Utilities|GetDPIScale)))) (Math|Float|Absolute(Float) (- -6.5e+02 (Variables|Default|GetheldDepth))))))) false false)))

(event Input|MouseEvents|LeftMouseButton
  (params (Key :type Key%20Structure))
  (bind _sb (Variables|Default|Getsb))
  (:Released
    (Variables|/Game/Blueprints/Switchboard_Blueprint.Switchboard_Blueprint_C|Setenabled (Variables|Default|Getsb) false)
    (if (Math|Boolean|ANDBoolean (Variables|Default|GetisPlugHeld) (Variables|Default|Getactive) (Variables|/Game/Blueprints/Switchboard_Blueprint.Switchboard_Blueprint_C|GetsocketSelected _sb))
      (Transformation|SetWorldLocation (Variables|Default|GetplugHeld) (+ (Variables|/Game/Blueprints/Switchboard_Blueprint.Switchboard_Blueprint_C|GetclosestSocketLocation3D _sb) "-20.000000,0.000000,-10.000000") false false))
    (Variables|Default|SetisPlugHeld false)
    (bind _letter (Default|Plug (Variables|Default|Getsb) self))
    (if (== (Variables|Default|GetplugHeld) (Variables|Default|Getplug1))
      (Variables|Default|Setplug1Letter _letter)
      (else
        (Variables|Default|Setplug2Letter _letter)))))

(fn ConstructionScript)

(fn GetEncoding
  (params (letter :type String))
  (bind _plug1letter (Variables|Default|Getplug1Letter))
  (bind _plug2letter (Variables|Default|Getplug2Letter))
  (if (Utilities|Enum|Equal(Enum) letter _plug1letter)
    (if (Utilities|Enum|Equal(Enum) _plug2letter "None")
      _
      (else
        (return _plug2letter)))
    (elif (Utilities|Enum|Equal(Enum) _plug1letter "None")
      _
      (else
        (return _plug1letter))))
  (return letter))