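; Keyboard controller Blueprint that maps physical letter keys A to Z onto matching button objects, one per letter.
; Each key press calls EventClick on its button, and each release calls EventWaitAndRelease on the same button.
; The wiring is repeated per key with no shared logic, and the construction script is empty.
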(event Input|KeyboardEvents|Z
  (params (Key :type Key%20Structure))
  (bind _z_button (Variables|Default|GetZ_Button))
  (:Pressed
    (Default|EventClick _z_button))
  (:Released
    (Default|EventWaitandRelease _z_button)))

(event Input|KeyboardEvents|A
  (params (Key :type Key%20Structure))
  (bind _a_button (Variables|Default|GetA_Button))
  (:Pressed
    (Default|EventClick _a_button))
  (:Released
    (Default|EventWaitandRelease _a_button)))

(event Input|KeyboardEvents|J
  (params (Key :type Key%20Structure))
  (bind _j_button (Variables|Default|GetJ_Button))
  (:Pressed
    (Default|EventClick _j_button))
  (:Released
    (Default|EventWaitandRelease _j_button)))

(event Input|KeyboardEvents|K
  (params (Key :type Key%20Structure))
  (bind _k_button (Variables|Default|GetK_Button))
  (:Pressed
    (Default|EventClick _k_button))
  (:Released
    (Default|EventWaitandRelease _k_button)))

(event Input|KeyboardEvents|L
  (params (Key :type Key%20Structure))
  (bind _l_button (Variables|Default|GetL_Button))
  (:Pressed
    (Default|EventClick _l_button))
  (:Released
    (Default|EventWaitandRelease _l_button)))

(event Input|KeyboardEvents|M
  (params (Key :type Key%20Structure))
  (bind _m_button (Variables|Default|GetM_Button))
  (:Pressed
    (Default|EventClick _m_button))
  (:Released
    (Default|EventWaitandRelease _m_button)))

(event Input|KeyboardEvents|N
  (params (Key :type Key%20Structure))
  (bind _n_button (Variables|Default|GetN_Button))
  (:Pressed
    (Default|EventClick _n_button))
  (:Released
    (Default|EventWaitandRelease _n_button)))

(event Input|KeyboardEvents|Q
  (params (Key :type Key%20Structure))
  (bind _q_button (Variables|Default|GetQ_Button))
  (:Pressed
    (Default|EventClick _q_button))
  (:Released
    (Default|EventWaitandRelease _q_button)))

(event Input|KeyboardEvents|O
  (params (Key :type Key%20Structure))
  (bind _o_button (Variables|Default|GetO_Button))
  (:Pressed
    (Default|EventClick _o_button))
  (:Released
    (Default|EventWaitandRelease _o_button)))

(event Input|KeyboardEvents|P
  (params (Key :type Key%20Structure))
  (bind _p_button (Variables|Default|GetP_Button))
  (:Pressed
    (Default|EventClick _p_button))
  (:Released
    (Default|EventWaitandRelease _p_button)))

(event Input|KeyboardEvents|R
  (params (Key :type Key%20Structure))
  (bind _r_button (Variables|Default|GetR_Button))
  (:Pressed
    (Default|EventClick _r_button))
  (:Released
    (Default|EventWaitandRelease _r_button)))

(event Input|KeyboardEvents|B
  (params (Key :type Key%20Structure))
  (bind _b_button (Variables|Default|GetB_Button))
  (:Pressed
    (Default|EventClick _b_button))
  (:Released
    (Default|EventWaitandRelease _b_button)))

(event Input|KeyboardEvents|S
  (params (Key :type Key%20Structure))
  (bind _s_button (Variables|Default|GetS_Button))
  (:Pressed
    (Default|EventClick _s_button))
  (:Released
    (Default|EventWaitandRelease _s_button)))

(event Input|KeyboardEvents|T
  (params (Key :type Key%20Structure))
  (bind _t_button (Variables|Default|GetT_Button))
  (:Pressed
    (Default|EventClick _t_button))
  (:Released
    (Default|EventWaitandRelease _t_button)))

(event Input|KeyboardEvents|U
  (params (Key :type Key%20Structure))
  (bind _u_button (Variables|Default|GetU_Button))
  (:Pressed
    (Default|EventClick _u_button))
  (:Released
    (Default|EventWaitandRelease _u_button)))

(event Input|KeyboardEvents|W
  (params (Key :type Key%20Structure))
  (bind _w_button (Variables|Default|GetW_Button))
  (:Pressed
    (Default|EventClick _w_button))
  (:Released
    (Default|EventWaitandRelease _w_button)))

(event Input|KeyboardEvents|V
  (params (Key :type Key%20Structure))
  (bind _v_button (Variables|Default|GetV_Button))
  (:Pressed
    (Default|EventClick _v_button))
  (:Released
    (Default|EventWaitandRelease _v_button)))

(event Input|KeyboardEvents|X
  (params (Key :type Key%20Structure))
  (bind _x_button (Variables|Default|GetX_Button))
  (:Pressed
    (Default|EventClick _x_button))
  (:Released
    (Default|EventWaitandRelease _x_button)))

(event Input|KeyboardEvents|Y
  (params (Key :type Key%20Structure))
  (bind _y_button (Variables|Default|GetY_Button))
  (:Pressed
    (Default|EventClick _y_button))
  (:Released
    (Default|EventWaitandRelease _y_button)))

(event Input|KeyboardEvents|C
  (params (Key :type Key%20Structure))
  (bind _c_button (Variables|Default|GetC_Button))
  (:Pressed
    (Default|EventClick _c_button))
  (:Released
    (Default|EventWaitandRelease _c_button)))

(event Input|KeyboardEvents|D
  (params (Key :type Key%20Structure))
  (bind _d_button (Variables|Default|GetD_Button))
  (:Pressed
    (Default|EventClick _d_button))
  (:Released
    (Default|EventWaitandRelease _d_button)))

(event Input|KeyboardEvents|E
  (params (Key :type Key%20Structure))
  (bind _e_button (Variables|Default|GetE_Button))
  (:Pressed
    (Default|EventClick _e_button))
  (:Released
    (Default|EventWaitandRelease _e_button)))

(event Input|KeyboardEvents|F
  (params (Key :type Key%20Structure))
  (bind _f_button (Variables|Default|GetF_Button))
  (:Pressed
    (Default|EventClick _f_button))
  (:Released
    (Default|EventWaitandRelease _f_button)))

(event Input|KeyboardEvents|G
  (params (Key :type Key%20Structure))
  (bind _g_button (Variables|Default|GetG_Button))
  (:Pressed
    (Default|EventClick _g_button))
  (:Released
    (Default|EventWaitandRelease _g_button)))

(event Input|KeyboardEvents|H
  (params (Key :type Key%20Structure))
  (bind _h_button (Variables|Default|GetH_Button))
  (:Pressed
    (Default|EventClick _h_button))
  (:Released
    (Default|EventWaitandRelease _h_button)))

(event Input|KeyboardEvents|I
  (params (Key :type Key%20Structure))
  (bind _i_button (Variables|Default|GetI_Button))
  (:Pressed
    (Default|EventClick _i_button))
  (:Released
    (Default|EventWaitandRelease _i_button)))

(fn ConstructionScript)