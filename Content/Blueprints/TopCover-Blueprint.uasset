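; TopCover Blueprint for a clickable cover that toggles between open and closed.
; A direct click acts only while open and a panel lock click only while closed, both feeding a shared toggle gated by the TopCover reference's IsOpen.
; The toggle flips IsOpen and calls the parent's open or close event.
; Cursor hover enables custom depth on the mesh while open, clearing it on exit.
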(event OnBeginCursorOver(StaticMeshComponent)
  (params (TouchedComponent :type Primitive%20Component%20Object%20Reference))
  (if (Variables|Default|GetisOpen)
    (Rendering|SetRenderCustomDepth TouchedComponent true)))

(event OnEndCursorOver(StaticMeshComponent)
  (params (TouchedComponent :type Primitive%20Component%20Object%20Reference))
  (Rendering|SetRenderCustomDepth TouchedComponent false))

(event Custom|PanelLockClicked_Event
  (bind _parent (Variables|Default|Getparent))
  (if (not (Variables|Default|GetisOpen))
    (if (Variables|/Game/Blueprints/case/CoverTop-Blueprint.CoverTop-Blueprint_C|GetisOpen (Variables|Default|GetTopCover))
      (if (Variables|Default|GetisOpen)
        (Variables|Default|SetisOpen false)
        (Default|CloseEvent _parent)
        (else
          (Variables|Default|SetisOpen true)
          (Default|OpenEvent _parent))))))

(event MouseInput|EventActorOnClicked
  (params (ButtonPressed :type Key%20Structure))
  (bind _parent (Variables|Default|Getparent))
  (if (Variables|Default|GetisOpen)
    (if (Variables|/Game/Blueprints/case/CoverTop-Blueprint.CoverTop-Blueprint_C|GetisOpen (Variables|Default|GetTopCover))
      (if (Variables|Default|GetisOpen)
        (Variables|Default|SetisOpen false)
        (Default|CloseEvent _parent)
        (else
          (Variables|Default|SetisOpen true)
          (Default|OpenEvent _parent))))))

(fn ConstructionScript)