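; GlassLetter is a Blueprint for a mesh, named as a glass letter, that switches between a lit and a dark look.
; It applies the dark material on BeginPlay.
; The EventLight event stores the requested state in IsLight and swaps the static mesh's first material slot to light or dark, but only when ShouldShine is true.
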(event Custom|EventLight
  (params (shouldLight :type Boolean))
  (if (Variables|Default|GetshouldShine)
    (bind _output_get (Variables|Default|SetisLight shouldLight))
    (if _output_get
      (CallFunction|SetMaterialLight)
      (else
        (CallFunction|SetMaterialDark)))))

(event EventBeginPlay
  (CallFunction|SetMaterialDark))

(fn ConstructionScript)

(fn SetMaterialDark
  (Rendering|Material|SetMaterial (Variables|Debug|GetStaticMeshComponent) 0 (Variables|Default|GetdarkMaterial)))

(fn SetMaterialLight
  (Rendering|Material|SetMaterial (Variables|Debug|GetStaticMeshComponent) 0 (Variables|Default|GetlightMaterial)))