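; Clip actor for a case that swings between a start and an end rotation as it opens and closes.
; Clicking its static mesh calls the open event on CoverTop rather than moving the clip directly.
; Its own open and close events set an IsOpen flag and play or reverse a timeline that lerps the actor's rotation, which starts at the closed pose on BeginPlay.
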(event OnClicked(StaticMeshComponent)
  (params (TouchedComponent :type Primitive%20Component%20Object%20Reference) (ButtonPressed :type Key%20Structure))
  (Default|OpenEvent (Variables|Default|GetcoverTop)))

(event Custom|openEvent
  (Variables|Default|SetisOpen true)
  (bind _newtrack_0 (Timeline|Timeline_0 Play)
    (:Update
      (Transformation|SetActorRotation (Math|Rotator|Lerp(Rotator) (Variables|Default|GetstartRotation) (Variables|Default|GetendRotation) _newtrack_0)))))

(event Custom|closeEvent
  (Variables|Default|SetisOpen false)
  (bind _newtrack_0 (Timeline|Timeline_0 Reverse)
    (:Update
      (Transformation|SetActorRotation (Math|Rotator|Lerp(Rotator) (Variables|Default|GetstartRotation) (Variables|Default|GetendRotation) _newtrack_0)))))

(event EventBeginPlay
  (Transformation|SetActorRotation (Variables|Default|GetstartRotation)))

(fn ConstructionScript)