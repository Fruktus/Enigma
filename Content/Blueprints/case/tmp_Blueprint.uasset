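; Temporary-named actor Blueprint that steps a hinge support animation forward each time the actor is clicked.
; Each click adds a fixed increment to an unclamped Tmp value and writes it to Pos on the HingeSupportAnimation instance of the referenced Anim skeletal mesh.
; An unconnected SetPosition call on a separate Hinge mesh never runs, and the construction script is empty.
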(event EventBeginPlay)

(event Collision|EventActorBeginOverlap
  (params (OtherActor :type Actor%20Object%20Reference)))

(event EventTick
  (params (DeltaSeconds :type Float%20%28single-precision%29)))

(event MouseInput|EventActorOnClicked
  (params (ButtonPressed :type Key%20Structure))
  (bind _output_get (Variables|Default|Settmp (+ (Variables|Default|Gettmp) 0.1)))
  (bind _ashinge_support_animation (Utilities|Casting|CastToHingeSupportAnimation (Components|SkeletalMesh|GetAnimInstance (Variables|/Script/Engine.SkeletalMeshActor|GetSkeletalMeshComponent (Variables|Default|Getanim)))))
  (Variables|/Game/EnigmaModels/Case/HingeSupportAnimation.HingeSupportAnimation_C|Setpos _ashinge_support_animation _output_get))

(fn ConstructionScript)