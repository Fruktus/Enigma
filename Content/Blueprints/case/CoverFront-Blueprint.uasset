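; Front cover of a case that toggles open and closed on click, but only while the top cover is open.
; A timeline lerps the actor's rotation between start and end rotators, playing to open and reversing to close.
; Linked hook Blueprints fire just before opening, with a short delay ahead of the swing, and again once closing finishes.
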(event Custom|openEvent
  (Variables|Default|SetisOpen true)
  (CallFunction|FireHooks)
  (Utilities|FlowControl|Delay 0.2)
  (bind _newtrack_0 (Timeline|Timeline_0 Play)
    (:Update
      (Transformation|SetActorRotation (Math|Rotator|Lerp(Rotator) (Variables|Default|GetstartRotation) (Variables|Default|GetendRotation) _newtrack_0)))
    (:Finished
      (if (not (Variables|Default|GetisOpen))
        (CallFunction|FireHooks)))))

(event Custom|closeEvent
  (Variables|Default|SetisOpen false)
  (bind _newtrack_0 (Timeline|Timeline_0 Reverse)
    (:Update
      (Transformation|SetActorRotation (Math|Rotator|Lerp(Rotator) (Variables|Default|GetstartRotation) (Variables|Default|GetendRotation) _newtrack_0)))
    (:Finished
      (if (not (Variables|Default|GetisOpen))
        (CallFunction|FireHooks)))))

(event Custom|FireHooks
  (for _array_element (Utilities|Struct|BreakArrayOfActor (Variables|Default|Gethooks))
    (bind _ashook__blueprint (Utilities|Casting|CastToHook-Blueprint _array_element))
    (Default|FireEvent _ashook__blueprint)))

(event EventBeginPlay
  (Transformation|SetActorRotation (Variables|Default|GetstartRotation)))

(event MouseInput|EventActorOnClicked
  (params (ButtonPressed :type Key%20Structure))
  (if (Variables|/Game/Blueprints/case/CoverTop-Blueprint.CoverTop-Blueprint_C|GetisOpen (Variables|Default|GetCoverTop))
    (if (Variables|Default|GetisOpen)
      (CallFunction|CloseEvent)
      (else
        (CallFunction|OpenEvent)))))

(fn ConstructionScript)