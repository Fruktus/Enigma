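; CoverTop is a clickable case lid that toggles open and closed, ignoring clicks while RotorsCover is open.
; Opening releases the Clip, then after a short delay plays a timeline that lerps the actor between start and end rotations.
; The same timeline drives the HingeSupport animation's Pos through a two-slope remap built with Max.
; Closing reverses the timeline and shuts the Clip when it finishes.
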(event Custom|openEvent
  (Variables|Default|SetisOpen true)
  (Default|OpenEvent (Variables|Default|Getclip))
  (Utilities|FlowControl|Delay 0.4)
  (bind _newtrack_0 (Timeline|Timeline_0 Play)
    (:Update
      (bind _ashinge_support_animation (Utilities|Casting|CastToHingeSupportAnimation (Components|SkeletalMesh|GetAnimInstance (Variables|/Script/Engine.SkeletalMeshActor|GetSkeletalMeshComponent (Variables|Default|GethingeSupport)))))
      (bind _output (CallFunction|NewFunction0 _newtrack_0))
      (Variables|/Game/EnigmaModels/Case/HingeSupportAnimation.HingeSupportAnimation_C|Setpos _ashinge_support_animation _output)
      (Transformation|SetActorRotation (Math|Rotator|Lerp(Rotator) (Variables|Default|GetstartRotation) (Variables|Default|GetendRotation) _newtrack_0 true)))
    (:Finished
      (if (not (Variables|Default|GetisOpen))
        (Default|CloseEvent (Variables|Default|Getclip))))))

(event Custom|closeEvent
  (Variables|Default|SetisOpen false)
  (bind _newtrack_0 (Timeline|Timeline_0 Reverse)
    (:Update
      (bind _ashinge_support_animation (Utilities|Casting|CastToHingeSupportAnimation (Components|SkeletalMesh|GetAnimInstance (Variables|/Script/Engine.SkeletalMeshActor|GetSkeletalMeshComponent (Variables|Default|GethingeSupport)))))
      (bind _output (CallFunction|NewFunction0 _newtrack_0))
      (Variables|/Game/EnigmaModels/Case/HingeSupportAnimation.HingeSupportAnimation_C|Setpos _ashinge_support_animation _output)
      (Transformation|SetActorRotation (Math|Rotator|Lerp(Rotator) (Variables|Default|GetstartRotation) (Variables|Default|GetendRotation) _newtrack_0 true)))
    (:Finished
      (if (not (Variables|Default|GetisOpen))
        (Default|CloseEvent (Variables|Default|Getclip))))))

(event EventBeginPlay
  (Transformation|SetActorRotation (Variables|Default|GetstartRotation)))

(event MouseInput|EventActorOnClicked
  (params (ButtonPressed :type Key%20Structure))
  (if (not (Variables|/Game/Blueprints/TopCover-Blueprint.TopCover-Blueprint_C|GetisOpen (Variables|Default|GetrotorsCover)))
    (if (Variables|Default|GetisOpen)
      (CallFunction|CloseEvent)
      (else
        (CallFunction|OpenEvent)))))

(fn ConstructionScript)

(fn NewFunction0
  (params (input :type Float%20%28single-precision%29))
  (return (Math|Float|Max(Float) (- (* input 1.8) 0.8) (* input 0.88))))