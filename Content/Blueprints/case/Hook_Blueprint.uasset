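; Hook actor that rotates between open and closed orientations and also reacts to mouse clicks.
; It snaps to StartRotation at BeginPlay, and fireEvent toggles IsOpen, playing or reversing one timeline that lerps between StartRotation and EndRotation.
; A click plays a separate timeline that pitches the actor toward a 359-degree offset, re-reading the current rotation on every update.
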(event Custom|openEvent
  (Variables|Default|SetisOpen true)
  (bind _newtrack_0 (Timeline|Timeline_0 Play)
    (:Update
      (Transformation|SetActorRotation (Math|Rotator|Lerp(Rotator) (Variables|Default|GetstartRotation) (Variables|Default|GetendRotation) _newtrack_0)))))

(event Custom|closeEvent
  (Variables|Default|SetisOpen false)
  (bind _newtrack_0 (Timeline|Timeline_0 Reverse)
    (:Update
      (Transformation|SetActorRotation (Math|Rotator|Lerp(Rotator) (Variables|Default|GetstartRotation) (Variables|Default|GetendRotation) _newtrack_0)))))

(event Custom|fireEvent
  (if (Variables|Default|GetisOpen)
    (CallFunction|CloseEvent)
    (else
      (CallFunction|OpenEvent))))

(event EventBeginPlay
  (Transformation|SetActorRotation (Variables|Default|GetstartRotation)))

(event Collision|EventActorBeginOverlap
  (params (OtherActor :type Actor%20Object%20Reference)))

(event EventTick
  (params (DeltaSeconds :type Float%20%28single-precision%29)))

(event MouseInput|EventActorOnClicked
  (params (ButtonPressed :type Key%20Structure))
  (bind _returnvalue (Transformation|GetActorRotation))
  (bind (_roll _pitch _yaw) (Math|Rotator|BreakRotator _returnvalue))
  (bind _newtrack_0 (Timeline|clickTimeline Play)
    (:Update
      (Transformation|SetActorRotation (Math|Rotator|Lerp(Rotator) _returnvalue (Math|Rotator|MakeRotator _roll (+ _pitch 359.0) _yaw) _newtrack_0)))))

(fn ConstructionScript)