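; Clip_Blueprint is an actor for a clip, filed under case assets, that swings between a closed and an open rotation.
; On BeginPlay it snaps to StartRotation.
; The openEvent and closeEvent events set IsOpen and play or reverse a timeline, whose track drives a rotation lerp toward EndRotation or back.
; Nothing in the graph triggers these events, and overlap and Tick are unused.
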(event Custom|openEvent
  (Variables|Default|SetisOpen true)
  (bind _newtrack_0 (Timeline|Timeline_0 Play)
    (:Update
      (Transformation|SetActorRotation (Math|Rotator|Lerp(Rotator) (Variables|Default|GetstartRotation) (Variables|Default|GetendRotation) _newtrack_0)))))

(event Custom|closeEvent
  (Variables|Default|SetisOpen false)
  (bind _newtrack_0 (Timeline|Timeline_0 Reverse)
    (:Update
      (Transformation|SetActorRotation (Math|Rotator|Lerp(Rotator) (Variables|Default|GetstartRotation) (Variables|Default|GetendRotation) _newtrack_0)))))

(event EventBeginPlay
  (Transformation|SetActorRotation (Variables|Default|GetstartRotation)))

(event Collision|EventActorBeginOverlap
  (params (OtherActor :type Actor%20Object%20Reference)))

(event EventTick
  (params (DeltaSeconds :type Float%20%28single-precision%29)))

(fn ConstructionScript)