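; Switchboard actor that finds the mesh socket under the mouse and provides a plug-based letter substitution lookup.
; Each tick it projects every socket to screen space and compares it with the DPI-scaled mouse position, saving a closer one within MinDistance as the selection.
; Debug boxes mark all sockets and the selected one.
; GetEncoding returns a letter's PlugMap partner, or the letter itself when unmapped.
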(event EventBeginPlay)

(event Collision|EventActorBeginOverlap
  (params (OtherActor :type Actor%20Object%20Reference)))

(event EventTick
  (params (DeltaSeconds :type Float%20%28single-precision%29))
  (bind _returnvalue (Class|WidgetLayoutLibrary|GetMousePositiononViewport))
  (Variables|Default|SetmousePos _returnvalue)
  ;[1 1 1] dbg
  (Development|PrintString (Utilities|String|ToString(Vector2d) (Variables|Default|GetclosestSocketLocation2D)) false true "(R=0.000000,G=0.660000,B=1.000000,A=1.000000)" 0.1)
  (Development|PrintString (Utilities|String|ToString(Vector2d) (Variables|Default|GetmousePos)) false true "(R=0.327522,G=0.000000,B=1.000000,A=1.000000)" 0.1)
  (for _array_element (Transformation|GetAllSocketNames (Variables|Debug|GetStaticMeshComponent))
    (Rendering|Debug|DrawDebugBox (Transformation|GetSocketLocation (Variables|Debug|GetStaticMeshComponent) _array_element) "10.000000,10.000000,10.000000" "(R=1.000000,G=0.000000,B=0.000000,A=1.000000)" "0, 0, 0" 0.05 1.0)
    (Rendering|Debug|DrawDebugBox (Variables|Default|GetclosestSocketLocation3D) "10.000000,10.000000,10.000000" "(R=0.000000,G=1.000000,B=0.049054,A=1.000000)" "0, 0, 0" 0.05 2.0)
    (Math|Float|CompareFloat (Math|Vector2D|Vector2DLength (- (* (Variables|Default|GetmousePos) (Utilities|GetDPIScale)) (.ScreenPosition (Class|GameplayStatics|ProjectWorldtoScreen (Game|GetPlayerController 0) (Transformation|GetSocketLocation (Variables|Debug|GetStaticMeshComponent) _array_element) false)))) (Math|Vector2D|Vector2DLength (- (Variables|Default|GetclosestSocketLocation2D) (* (Variables|Default|GetmousePos) (Utilities|GetDPIScale))))
      (:<
        (Math|Float|CompareFloat (Math|Vector2D|Vector2DLength (- (* (Variables|Default|GetmousePos) (Utilities|GetDPIScale)) (.ScreenPosition (Class|GameplayStatics|ProjectWorldtoScreen (Game|GetPlayerController 0) (Transformation|GetSocketLocation (Variables|Debug|GetStaticMeshComponent) _array_element) false)))) (Variables|Default|GetminDistance)
          (:>
            (Variables|Default|SetclosestSocketLocation3D "0, 0, 0")
            (Variables|Default|SetsocketSelected false))
          (:==
            (Variables|Default|SetclosestSocketLocation2D (.ScreenPosition (Class|GameplayStatics|ProjectWorldtoScreen (Game|GetPlayerController 0) (Transformation|GetSocketLocation (Variables|Debug|GetStaticMeshComponent) _array_element) false)) :!label _label)
            (Variables|Default|SetsocketSelected true)
            (Variables|Default|SetclosestSocketLocation3D (Transformation|GetSocketLocation (Variables|Debug|GetStaticMeshComponent) _array_element))
            (bind _output_get (Variables|Default|SetclosestSocketName _array_element))
            (Development|PrintString (Utilities|String|ToString(Name) _output_get) false))
          (:<
            (goto _label))))))
  (Utilities|FlowControl|Delay 5.0))

(fn ConstructionScript)

(fn GetEncoding
  (params (inLetter :type String))
  (bind _plugmap (Variables|Default|GetplugMap))
  (bind (_value _returnvalue) (Utilities|Map|Find _plugmap inLetter))
  (if _returnvalue
    (return _value)
    (else
      (return inLetter))))