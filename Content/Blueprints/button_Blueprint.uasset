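; Clickable key actor that sends its letter to an EncryptionController when pressed, likely as part of a cipher machine keyboard.
; A click plays a pitch-randomized sound and a timeline that offsets the key vertically, with IsRunning blocking re-triggers.
; Mouse release or cursor exit clears the custom depth render and queues a release.
; Two flags delay the key-up sound and reversed timeline until the press animation finishes.
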(event Custom|EventClickAnimation
  (Variables|Default|SetisPlayingClickAnimation true)
  (bind _newtrack_8 (Timeline|ButtonTimeline Play)
    (:Update
      (Transformation|SetActorLocation (+ (Variables|Default|GetstartLocation) (Math|Vector|MakeVector 0.0 0.0 _newtrack_8)) false false))
    (:Finished
      (if (Variables|Default|GetisPlayingClickAnimation)
        (Variables|Default|SetisClicked true)
        (CallFunction|EventTryRelease)
        (else
          (Variables|Default|SetisRunning false))))))

(event Custom|EventReleaseAnimation
  (Variables|Default|SetisPlayingClickAnimation false)
  (bind _newtrack_8 (Timeline|ButtonTimeline Reverse)
    (:Update
      (Transformation|SetActorLocation (+ (Variables|Default|GetstartLocation) (Math|Vector|MakeVector 0.0 0.0 _newtrack_8)) false false))
    (:Finished
      (if (Variables|Default|GetisPlayingClickAnimation)
        (Variables|Default|SetisClicked true)
        (CallFunction|EventTryRelease)
        (else
          (Variables|Default|SetisRunning false))))))

(event Custom|EventWaitAndRelease
  (if (Variables|Default|GetisPlayingClickAnimation)
    (Variables|Default|SetshouldBeReleased true)
    (CallFunction|EventTryRelease)))

(event Custom|Event%20Try%20Release
  (if (and (Variables|Default|GetisClicked) (Variables|Default|GetshouldBeReleased))
    (Variables|Default|SetisClicked false)
    (Variables|Default|SetshouldBeReleased false)
    (CallFunction|EventRelease)))

(event Custom|EventClick
  (if (not (Variables|Default|GetisRunning))
    (Variables|Default|SetisRunning true)
    (Audio|PlaySound2D "/Game/Sounds/key-down.key-down" 1.0 (Math|Random|RandomFloatinRange 0.85 1.15) 0.0 0 0)
    (CallFunction|EventClickAnimation)
    (Class|EncryptionController|EncryptLetter (Variables|Default|GetEncryptionController) (Variables|Default|GetLetter))))

(event Custom|EventRelease
  (Audio|PlaySound2D "/Game/Sounds/key-up.key-up" 1.0 (Math|Random|RandomFloatinRange 0.85 1.15) 0.0 0 0)
  (CallFunction|EventReleaseAnimation))

(event MouseInput|EventActorEndCursorOver
  (CallFunction|EventWaitandRelease)
  (Rendering|SetRenderCustomDepth (Variables|Debug|GetStaticMeshComponent) false))

(event EventBeginPlay
  (Variables|Default|SetstartLocation (Transformation|GetActorLocation)))

(event MouseInput|EventActorOnClicked
  (params (ButtonPressed :type Key%20Structure))
  (CallFunction|EventClick))

(event EventActorOnReleased
  (params (ButtonReleased :type Key%20Structure))
  (CallFunction|EventWaitandRelease)
  (Rendering|SetRenderCustomDepth (Variables|Debug|GetStaticMeshComponent) false))

(fn ConstructionScript)