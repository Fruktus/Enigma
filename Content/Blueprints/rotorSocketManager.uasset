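; Manager actor that picks the rotor socket nearest the mouse cursor and attaches a rotor to it on request.
; It gathers three socket references on BeginPlay; while Active, Tick projects free sockets to screen space and keeps whichever beats the stored closest position's cursor distance.
; Debug boxes mark free sockets and the current pick.
; AttachToSelected hands the given rotor to that closest socket.
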(event EventBeginPlay
  (Utilities|Array|Add (Variables|Default|GetsocketArray) (Variables|Default|Getsocket1))
  (Utilities|Array|Add (Variables|Default|GetsocketArray) (Variables|Default|Getsocket2))
  (Utilities|Array|Add (Variables|Default|GetsocketArray) (Variables|Default|Getsocket3)))

(event Collision|EventActorBeginOverlap
  (params (OtherActor :type Actor%20Object%20Reference)))

(event EventTick
  (params (DeltaSeconds :type Float%20%28single-precision%29))
  (if (Variables|Default|Getactive)
    (for _array_element (Variables|Default|GetsocketArray)
      (if (Variables|/Game/Blueprints/rotorSocket.rotorSocket_C|GetisFree _array_element)
        ;[1 1 1] dbg
        (Rendering|Debug|DrawDebugBox (Transformation|GetActorLocation _array_element) "10.000000,10.000000,10.000000" "(R=1.000000,G=0.000000,B=0.279033,A=1.000000)" "0, 0, 0" 0.2 1.0)
        (bind _returnvalue (Class|WidgetLayoutLibrary|GetMousePositiononViewport))
        (Math|Float|CompareFloat (Math|Vector2D|Vector2DLength (- _returnvalue (.ScreenPosition (Class|GameplayStatics|ProjectWorldtoScreen (Game|GetPlayerController 0) (Transformation|GetActorLocation _array_element) false)))) (Math|Vector2D|Vector2DLength (- _returnvalue (Variables|Default|GetclosestSocketLocation)))
          (:<
            (Variables|Default|SetclosestSocketLocation (.ScreenPosition (Class|GameplayStatics|ProjectWorldtoScreen (Game|GetPlayerController 0) (Transformation|GetActorLocation _array_element) false)))
            (Variables|Default|SetclosestSocket _array_element)))))
    (Utilities|FlowControl|Delay 0.2)
    ;[1 1 1] dbg
    (Rendering|Debug|DrawDebugBox (Transformation|GetActorLocation (Variables|Default|GetclosestSocket)) "10.000000,10.000000,10.000000" "(R=0.000000,G=1.000000,B=0.211516,A=1.000000)" "0, 0, 0" 0.2 2.0)))

(fn ConstructionScript)

(fn AttachtoSelected
  (params (rotor :type Rotor%20Assembly%20Blueprint%20Object%20Reference))
  (Default|Attach (Variables|Default|GetclosestSocket) rotor))