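; Clickable rotor actor with 26 positions that the player turns by dragging the mouse while Enabled is set.
; Tick turns drag distance from the click point, in steps of 4% of viewport height, into an index modulo 26.
; An index change plays a timeline that sets pitch relative to the starting rotation, lerping between the raw index and Step × LastPos.
; LastPos updates on every timeline update and resets on release.
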(event OnClicked(Cube)
  (params (TouchedComponent :type Primitive%20Component%20Object%20Reference) (ButtonPressed :type Key%20Structure))
  (Variables|Default|Setis_left_down true)
  (bind _returnvalue (Class|WidgetLayoutLibrary|GetMousePositiononViewport))
  (Variables|Default|Setmouse_starting_pos _returnvalue))

(event OnReleased(Cube)
  (params (TouchedComponent :type Primitive%20Component%20Object%20Reference) (ButtonReleased :type Key%20Structure))
  (Variables|Default|Setis_left_down false)
  (Variables|Default|SetlastPos 0.0))

(event EventBeginPlay
  (Variables|Default|SetstartRotation (Transformation|GetActorRotation)))

(event Collision|EventActorBeginOverlap
  (params (OtherActor :type Actor%20Object%20Reference)))

(event EventTick
  (params (DeltaSeconds :type Float%20%28single-precision%29))
  (bind _startrotation (Variables|Default|GetstartRotation))
  (bind (_roll _pitch _yaw) (Math|Rotator|BreakRotator _startrotation))
  (if (and (Variables|Default|Getis_left_down) (Variables|Default|Getenabled))
    (bind _returnvalue (Class|WidgetLayoutLibrary|GetMousePositiononViewport))
    (if (not (== (Math|Float|%(Float) (Math|Conversions|ToFloat(Integer) (Math|Float|Truncate (/ (Math|Vector2D|Vector2DLength (- _returnvalue (Variables|Default|Getmouse_starting_pos))) (* (.y (Viewport|GetViewportSize)) 0.04)))) (Math|Conversions|ToFloat(Integer) 26)) (Variables|Default|GetlastPos)))
      (bind _newtrack_0 (Timeline|Timeline_0 Play)
        (:Update
          (Transformation|SetActorRotation (Math|Rotator|MakeRotator _roll (+ (Math|Float|Lerp (Math|Float|%(Float) (Math|Conversions|ToFloat(Integer) (Math|Float|Truncate (/ (Math|Vector2D|Vector2DLength (- _returnvalue (Variables|Default|Getmouse_starting_pos))) (* (.y (Viewport|GetViewportSize)) 0.04)))) (Math|Conversions|ToFloat(Integer) 26)) (* (Variables|Default|Getstep) (Variables|Default|GetlastPos)) _newtrack_0) _pitch) _yaw))
          (Variables|Default|SetlastPos (Math|Float|%(Float) (Math|Conversions|ToFloat(Integer) (Math|Float|Truncate (/ (Math|Vector2D|Vector2DLength (- _returnvalue (Variables|Default|Getmouse_starting_pos))) (* (.y (Viewport|GetViewportSize)) 0.04)))) (Math|Conversions|ToFloat(Integer) 26))))))))

(event Input|MouseEvents|LeftMouseButton
  (params (Key :type Key%20Structure))
  (:Released
    (Variables|Default|Setis_left_down false)
    (Variables|Default|SetlastPos 0.0)))

(fn ConstructionScript
  (Variables|Default|Setstep (/ 3.6e+02 26.0)))