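; Lamp Blueprint for a single lettered lamp that lights up in response to an encryption controller.
; On BeginPlay it binds to the EncryptionController's lamp on and off events.
; Each handler ignores letters other than its own LampLetter, then sets the Center component's visibility and forwards the state to GlassLetter.
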(event Custom|onLightLampOn
  (params (letter :type ELetter%20Enum :default "A"))
  (if (CallFunction|ShouldContinue letter)
    (CallFunction|SetLight true)))

(event Custom|onLightLampOff
  (params (letter :type ELetter%20Enum :default "A"))
  (if (CallFunction|ShouldContinue letter)
    (CallFunction|SetLight false)))

(event EventBeginPlay
  (bind _encryptioncontroller (Variables|Default|GetEncryptionController))
  (EventDispatchers|BindEventtoOnLightLampon _encryptioncontroller (delegate Custom|onLightLampOn))
  (EventDispatchers|BindEventtoOnLightLampOff _encryptioncontroller (delegate Custom|onLightLampOff)))

(fn ConstructionScript)

(fn ToggleLight
  (Rendering|ToggleVisibility (Variables|Default|GetCenter) false)
  (Default|EventLight (Variables|Default|GetglassLetter) false))

(fn ShouldContinue
  (params (letter :type ELetter%20Enum :default "A"))
  (return (Utilities|Enum|Equal(Enum) letter (Variables|Default|GetLampLetter))))

(fn SetLight
  (params (lightOn :type Boolean))
  (Rendering|SetVisibility (Variables|Default|GetCenter) lightOn false)
  (Default|EventLight (Variables|Default|GetglassLetter) lightOn))