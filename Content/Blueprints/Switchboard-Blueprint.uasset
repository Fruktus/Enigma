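; Switchboard plugboard with lettered sockets that encodes letters through the cables plugged into them.
; While enabled, Tick projects free mesh sockets to screen space, picks the one nearest the DPI-scaled mouse, and spotlights it within a distance threshold.
; Plug and Unplug maintain a letter-to-cable map keyed by the socket name's first character.
; GetEncoding defers to the mapped cable, returning unplugged letters unchanged.
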(event EventBeginPlay)

(event Collision|EventActorBeginOverlap
  (params (OtherActor :type Actor%20Object%20Reference)))

(event EventTick
  (params (DeltaSeconds :type Float%20%28single-precision%29))
  (if (Variables|Default|Getenabled)
    (bind _returnvalue (Class|WidgetLayoutLibrary|GetMousePositiononViewport))
    (Variables|Default|SetmousePos _returnvalue)
    (for _array_element (Transformation|GetAllSocketNames (Variables|Debug|GetStaticMeshComponent))
      (if (not (Utilities|Map|Contains (Variables|Default|GetletterCableMap) (Utilities|String|ToString(Name) _array_element)))
        (Math|Float|CompareFloat (Math|Vector2D|Vector2DLength (- (* (Variables|Default|GetmousePos) (Utilities|GetDPIScale)) (.ScreenPosition (Class|GameplayStatics|ProjectWorldtoScreen (Game|GetPlayerController 0) (Transformation|GetSocketLocation (Variables|Debug|GetStaticMeshComponent) _array_element) false)))) (Math|Vector2D|Vector2DLength (- (Variables|Default|GetclosestSocketLocation2D) (* (Variables|Default|GetmousePos) (Utilities|GetDPIScale))))
          (:<
            (Variables|Default|SetclosestSocketLocation2D (.ScreenPosition (Class|GameplayStatics|ProjectWorldtoScreen (Game|GetPlayerController 0) (Transformation|GetSocketLocation (Variables|Debug|GetStaticMeshComponent) _array_element) false)))
            (Variables|Default|SetsocketSelected true)
            (Variables|Default|SetclosestSocketLocation3D (Transformation|GetSocketLocation (Variables|Debug|GetStaticMeshComponent) _array_element))
            (Variables|Default|SetclosestSocketName _array_element)))))
    (Math|Float|CompareFloat (Math|Vector2D|Vector2DLength (- (* (Variables|Default|GetmousePos) (Utilities|GetDPIScale)) (Variables|Default|GetclosestSocketLocation2D))) (Variables|Default|GetminDistance)
      (:>
        (Variables|Default|SetclosestSocketLocation3D "0, 0, 0" :!label _label)
        (Variables|Default|SetsocketSelected false)
        (Rendering|SetVisibility (Variables|/Script/Engine.SpotLight|GetSpotLightComponent (Variables|Default|Getspotlight)) false false))
      (:==
        (goto _label))
      (:<
        (Transformation|SetActorLocation (Variables|Default|Getspotlight) (Math|Vector|MakeVector (Variables|Default|GetlightDepth) (.y (Variables|Default|GetclosestSocketLocation3D)) (.z (Variables|Default|GetclosestSocketLocation3D))) false false)
        (Rendering|SetVisibility (Variables|/Script/Engine.SpotLight|GetSpotLightComponent (Variables|Default|Getspotlight)) true false)))
    (Utilities|FlowControl|Delay 5.0)
    (else
      (Rendering|SetVisibility (Variables|/Script/Engine.Light|GetLightComponent (Variables|Default|Getspotlight)) false false)
      (Utilities|FlowControl|Delay 5.0))))

(fn ConstructionScript)

(fn GetEncoding
  (params (inLetter :type String))
  (bind _lettercablemap (Variables|Default|GetletterCableMap))
  (bind (_value _returnvalue) (Utilities|Map|Find _lettercablemap inLetter))
  (if _returnvalue
    ;[1 1 1] Reverse lookup through cable
    (Default|GetEncoding _value inLetter)
    (else
      (return inLetter))))

(fn Plug
  (params (cable :type Cable-Blueprint%20Object%20Reference))
  (bind _closestsocketname (Variables|Default|GetclosestSocketName))
  (bind _returnvalue (Utilities|String|ToString(Name) _closestsocketname))
  (bind _returnvalue_2 (Utilities|String|GetSubstring _returnvalue 0))
  (Utilities|Map|Add (Variables|Default|GetletterCableMap) _returnvalue_2 cable)
  (return _returnvalue_2))

(fn Unplug
  (params (letter :type String))
  (Utilities|Map|Remove (Variables|Default|GetletterCableMap) letter))

(fn GetEnumEncoding
  (params (inputEnum :type ELetter%20Enum :default "A"))
  (CallFunction|GetEncoding (Utilities|String|EnumtoString inputEnum))
  (return "A"))

(fn LettertoSocketName
  (params (letter :type String))
  (return (Utilities|String|StringToName (Utilities|String|Append letter "_Socket"))))