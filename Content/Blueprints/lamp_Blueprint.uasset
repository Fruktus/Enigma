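; A lamp Blueprint that flashes when its assigned letter is lit, apparently one lamp in an encryption machine's lampboard.
; On BeginPlay it binds to the EncryptionController's OnLightLamp dispatcher.
; When the broadcast letter matches its LampLetter, it toggles the Center component's visibility and calls EventLight on GlassLetter, then repeats the toggle after a short delay to switch back.
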(event Custom|onLightLamp
  (params (letter :type ELetter%20Enum :default "A"))
  (if (Utilities|Enum|Equal(Enum) letter (Variables|Default|GetLampLetter))
    (CallFunction|ToggleLight)
    (Utilities|FlowControl|Delay 0.8)
    (CallFunction|ToggleLight)))

(event EventBeginPlay
  (EventDispatchers|AssignOnLightLamp (Variables|Default|GetEncryptionController) (delegate Custom|onLightLamp)))

(fn ConstructionScript)

(fn ToggleLight
  (Rendering|ToggleVisibility (Variables|Default|GetCenter) false)
  (Default|EventLight (Variables|Default|GetglassLetter)))